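; Player controller that shows the mouse cursor, enables click events and manages switching the view between the player pawn's camera and its AI pawn camera.
; BeginPlay sets the view to the pawn's ActiveCamera.
; The SwitchCamera event and a debug Space Bar key share one path that fires a camera-switch dispatcher, then uses a FlipFlop to alternate cameras with an eased blend and update ActiveCamera.
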(event `self.ReceiveBeginPlay`
  (set `self.bShowMouseCursor` true)
  (set `self.bEnableClickEvents` true)
  (bind _asppawn (cast `/Game/Blueprints/Actors/PPawn` (`self.K2_GetPawn`)))
  (`self.SetViewTargetWithBlend` (`/Game/Blueprints/Actors/PPawn.ActiveCamera` _asppawn)))

(event `Key|SpaceBar`
  (params (Key :type "Key Structure"))
  (:`Pressed`
    (`self.CameraSwitchDispatch` :!label _label)
    (bind _asppawn (cast `/Game/Blueprints/Actors/PPawn` (`self.K2_GetPawn`)))
    (`/Engine/EditorBlueprintResources/StandardMacros.FlipFlop`
      (:`A`
        (bind _childactor (`ChildActorComponent.ChildActor` (`/Game/Blueprints/Actors/AIPawn.CameraCloseup` (`/Game/Blueprints/Actors/PPawn.AIPawn` _asppawn))))
        (`self.SetViewTargetWithBlend` _childactor 1.0 "VTBlend_EaseOut" 0.5)
        (bind _ascamera_actor (cast `CameraActor` _childactor))
        (set `/Game/Blueprints/Actors/PPawn.ActiveCamera` _ascamera_actor _asppawn))
      (:`B`
        (bind _childactor_2 (`ChildActorComponent.ChildActor` (`/Game/Blueprints/Actors/PPawn.Camera` _asppawn)))
        (`self.SetViewTargetWithBlend` _childactor_2 1.0 "VTBlend_EaseOut" 0.5)
        (bind _ascamera_actor_2 (cast `CameraActor` _childactor_2))
        (set `/Game/Blueprints/Actors/PPawn.ActiveCamera` _ascamera_actor_2 _asppawn)))))

(event `Switch Camera`
  (goto _label))

(fn `UserConstructionScript`)