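; Base game mode for Java Jungle that handles level loading, player progress saving and background music.
; Loads levels by index from a list, records the current index on the game instance, and also opens the menu and victory screens.
; Save reads lazily load or create a PlayerProgressSave, with loaded data cached until the next write.
; Music starts once as a looping 2D sound, with volume taken from saved user settings.
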(event `self.ReceiveBeginPlay`)

(event `self.Music.OnAudioFinished`
  ;[1 1 1] Loop music track
  (`AudioComponent.Play` (`self.Music`) 0.0))

(fn `LoadLevel`
  (params (`Level Index` :type Integer))
  (if (> `Level Index` (`KismetArrayLibrary.Array_Length` (`self.LevelListArray`)))
    (`GameplayStatics.OpenLevel` "MainMenu") ; Return to menu if bad level
    (else
      (`GameplayStatics.OpenLevel` (`|GetArrayItem` (`self.LevelListArray`) `Level Index`))
      (bind _asjava_jungle_game_instance (cast `/Game/Blueprints/JavaJungleGameInstance` (`GameplayStatics.GetGameInstance`)))
      (set `/Game/Blueprints/JavaJungleGameInstance.CurrentLevelIndex` `Level Index` _asjava_jungle_game_instance))))

(fn `LoadMenu`
  (`GameplayStatics.OpenLevel` "MainMenu"))

(fn `LoadVictory`
  (`GameplayStatics.OpenLevel` "VictoryScreen"))

(fn `PlayMusic`
  (params (Music :type "SoundCue Object Reference"))
  (if (not (`self.MusicPlaying`))
    (bind _returnvalue (`GameplayStatics.CreateSound2D` Music 1.0 1.0 0.0 null))
    (bind _output_get (set `self.Music` _returnvalue))
    (`AudioComponent.Play` _output_get 0.0)
    (`self.ValidateVolume`)
    (set `self.MusicPlaying` true)))

(fn `ReadSaveData`
  (params (`Force validation` :type Boolean))
  (returns (`Save Data` :type "/Game/Blueprints/PlayerProgressSave Object Reference"))
  (bind (_saveslot _playerid) (defaults `/Game/Blueprints/PlayerProgressSave` "/Game/Blueprints/PlayerProgressSave.PlayerProgressSave_C"))
  (if (not (or `Force validation` (`self.SaveDataLoaded`)))
    (bind _returnvalue (`GameplayStatics.DoesSaveGameExist` _saveslot _playerid))
    (if _returnvalue
      (bind _returnvalue_2 (`GameplayStatics.LoadGameFromSlot` _saveslot _playerid))
      (bind _asplayer_progress_save (cast `/Game/Blueprints/PlayerProgressSave` _returnvalue_2))
      (set `self.SaveData` _asplayer_progress_save)
      (set `self.SaveDataLoaded` true)
      (else
        (bind _returnvalue_3 (`GameplayStatics.CreateSaveGameObject` "/Game/Blueprints/PlayerProgressSave.PlayerProgressSave_C"))
        (set `self.SaveData` _returnvalue_3))))
  (return (`self.SaveData`)))

(fn `SetLevelCompletion`
  (params (LevelName :type Name) (CompletionStatus :type Boolean))
  (locals (LevelCompletionMapTemp :type "Map of Name to Boolean"))
  (bind _save_data (`self.ReadSaveData` false))
  (`BlueprintMapLibrary.Map_Add` (`/Game/Blueprints/PlayerProgressSave.LevelCompletionMap` _save_data) LevelName CompletionStatus)
  (`self.WriteSaveData` _save_data))

(fn `UserConstructionScript`)

(fn `ValidateVolume`
  (bind _save_data (`self.ReadSaveData` false))
  (`AudioComponent.AdjustVolume` (`self.Music`) 0.0 (`self.Get user settings from save` _save_data)))

(fn `WriteSaveData`
  (params (`Save Data` :type "/Game/Blueprints/PlayerProgressSave Object Reference"))
  (`GameplayStatics.SaveGameToSlot` `Save Data` (`/Game/Blueprints/PlayerProgressSave.SaveSlot` `Save Data`) (`/Game/Blueprints/PlayerProgressSave.PlayerID` `Save Data`))
  (set `self.SaveDataLoaded` false))