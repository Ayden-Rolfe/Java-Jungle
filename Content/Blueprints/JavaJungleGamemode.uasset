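; Game mode for a Java Jungle level that tracks remaining beans and handles level completion.
; On BeginPlay it finds the player pawn, AI pawn and beans, wires references, HUD and camera into the player pawn, then starts music.
; UpdateBeanCounter decrements the count and notifies the player pawn.
; At zero it records completion, fades music, then after a delay loads victory on the final level or otherwise the menu.
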(event `self.ReceiveBeginPlay`
  ;[1 1 1] Get & Set necessary variables for all involved actors & load volume data
  (`|ExecutionSequence`
    (:`then_0`
      (bind _outactors (`GameplayStatics.GetAllActorsOfClass` "/Game/Blueprints/Actors/PPawn.PPawn_C"))
      (bind _output_get (set `self.PlayerPawn` (`|GetArrayItem` _outactors)))
      (bind _outactors_2 (`GameplayStatics.GetAllActorsOfClass` "/Game/Blueprints/Actors/Bean.Bean_C"))
      (set `self.BeanCount` (`KismetArrayLibrary.Array_Length` _outactors_2))
      (set `/Game/Blueprints/Actors/PPawn.Beans` _outactors_2 _output_get)
      (bind _outactors_3 (`GameplayStatics.GetAllActorsOfClass` "/Game/Blueprints/Actors/AIPawn.AIPawn_C"))
      (bind _output (`|GetArrayItem` _outactors_3))
      (set `self.AIPawn` _output)
      (set `/Game/Blueprints/Actors/PPawn.AIPawn` _output _output_get)
      (bind _returnvalue (`|CreateWidget` "/Game/Blueprints/GUI/Game_HUD.Game_HUD_C"))
      (bind _output_get_2 (set `/Game/Blueprints/Actors/PPawn.HUD` _returnvalue _output_get))
      (`UserWidget.AddToViewport` _output_get_2 0)
      (set `/Game/Blueprints/Actors/PPawn.AIPawn` (`self.AIPawn`) _output_get)
      (bind _ascamera_actor (cast `CameraActor` (`ChildActorComponent.ChildActor` (`/Game/Blueprints/Actors/PPawn.Camera` _output_get))))
      (set `/Game/Blueprints/Actors/PPawn.ActiveCamera` _ascamera_actor _output_get))
    (:`then_1`
      (`self.PlayMusic` "/Game/Sounds/Music/LevelMusic_Cue.LevelMusic_Cue"))))

(event `Update Bean Counter`
  (bind _result (`/Engine/EditorBlueprintResources/StandardMacros.DecrementInt` (`self.BeanCount`))
    (:`  `
      (bind _returnvalue (> _result 0))
      (`/Game/Blueprints/Actors/PPawn.Bean Decremented` (`self.PlayerPawn`) _returnvalue)
      (if (not _returnvalue)
        (bind _returnvalue_2 (`GameplayStatics.GetCurrentLevelName` true))
        (`self.SetLevelCompletion` (`KismetStringLibrary.Conv_StringToName` _returnvalue_2) true)
        (bind _asjava_jungle_gamemode_base (cast `/Game/Blueprints/JavaJungleGamemodeBase` (`GameplayStatics.GetGameMode`)))
        (`AudioComponent.FadeOut` (`/Game/Blueprints/JavaJungleGamemodeBase.Music` _asjava_jungle_gamemode_base) 2.0 0.0)
        (`KismetSystemLibrary.Delay` 3.0)
        (if (`self.IsFinalLevel`)
          (`self.LoadVictory` _asjava_jungle_gamemode_base)
          (else
            (`self.LoadMenu` _asjava_jungle_gamemode_base)))))))

(fn `UserConstructionScript`)