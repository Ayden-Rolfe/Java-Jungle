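; Bean is a spinning collectible pickup actor for the Java Jungle game mode.
; Tick rotates its root around yaw at a steady, frame-rate-independent speed.
; When an AIPawn overlaps it, it spawns a pooled pickup particle at the sparkles component, tells JavaJungleGamemode to update the bean counter, then destroys itself.
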(event `self.ReceiveActorBeginOverlap`
  (params (OtherActor :type "Actor Object Reference"))
  (cast `/Game/Blueprints/Actors/AIPawn` OtherActor)
  (bind _asjava_jungle_gamemode (cast `/Game/Blueprints/JavaJungleGamemode` (`GameplayStatics.GetGameMode`)))
  (`GameplayStatics.SpawnEmitterAtLocation` "/Game/ParticleSystems/Beanget/P_Bean_get.P_Bean_get" (`SceneComponent.K2_GetComponentLocation` (`self.BeanSparkles`)) (struct) (1.0 1.0 1.0) true "AutoRelease")
  (`/Game/Blueprints/JavaJungleGamemode.Update Bean Counter` _asjava_jungle_gamemode)
  (`self.K2_DestroyActor`))

(event `self.ReceiveTick`
  (params (DeltaSeconds :type "Float (single-precision)"))
  (`SceneComponent.K2_AddLocalRotation` (`self.Root`) (`KismetMathLibrary.MakeRotator` 0.0 0.0 (* 100 DeltaSeconds)) false false))

(fn `UserConstructionScript`)