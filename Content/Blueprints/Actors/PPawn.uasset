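; Player input pawn that steers a separate AI-controlled character across land tiles and pushable boxes.
; Clicks and single taps trace from the camera to pick walk targets, while keys and swipes trace one step in a compass direction, or push a grabbed box.
; A delayed tap counter detects double taps to switch cameras.
; Bean count changes update the HUD, and running out blocks character movement.
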(event `self.ReceiveBeginPlay`)

(event `InputAction|Instruct`
  (params (Key :type "Key Structure"))
  (:`Pressed`
    (`self.Movement Allowed Check`)
    (bind _asplayer_controller (cast `PlayerController` (`self.GetController`)))
    (bind (_worldlocation _worlddirection) (`PlayerController.DeprojectMousePositionToWorld` _asplayer_controller))
    (bind _hit (`self.Camera Trace` _worldlocation _worlddirection))
    (`self.Perform Move` _hit (`self.AIPawn`) "CD_North" false)))

(event `InputAction|MoveRight`
  (params (Key :type "Key Structure"))
  (:`Pressed`
    (`self.Movement Allowed Check`)
    (`self.CallMove` "CD_East")))

(event `InputAction|MoveLeft`
  (params (Key :type "Key Structure"))
  (:`Pressed`
    (`self.Movement Allowed Check`)
    (`self.CallMove` "CD_West")))

(event `InputAction|MoveUp`
  (params (Key :type "Key Structure"))
  (:`Pressed`
    (`self.Movement Allowed Check`)
    (`self.CallMove` "CD_North")))

(event `InputAction|MoveDown`
  (params (Key :type "Key Structure"))
  (:`Pressed`
    (`self.Movement Allowed Check`)
    (`self.CallMove` "CD_South")))

(event `InputTouch`
  (params (Location :type "Vector Structure") (FingerIndex :type "ETouchIndex Enum"))
  (bind (_worldlocation _worlddirection) (`PlayerController.DeprojectScreenPositionToWorld` (`GameplayStatics.GetPlayerController` 0) (.x Location) (.y Location)))
  (bind _returnvalue (- Location (`self.TouchStartPos`)))
  (bind _x (.x (`KismetMathLibrary.Normal` _returnvalue)))
  (bind _y (.y (`KismetMathLibrary.Normal` _returnvalue)))
  (:`Pressed`
    (set `self.TouchStartPos` Location))
  (:`Released`
    (`self.Movement Allowed Check`)
    (if (>= (`KismetMathLibrary.VSizeSquared` _returnvalue) (`KismetMathLibrary.Square` (`self.TapThreshold`)))
      (if (> (`KismetMathLibrary.Abs` _x) (`KismetMathLibrary.Abs` _y))
        (if (> _x 0.0)
          (`self.CallMove` "CD_East")
          (else
            (`self.CallMove` "CD_West")))
        (elif (< _y 0.0)
          (`self.CallMove` "CD_North")
          (else
            (`self.CallMove` "CD_South"))))
      (else
        (`self.TapCountRecogniser`
          (:`Single`
            (bind _hit (`self.Camera Trace` _worldlocation _worlddirection))
            (`self.Perform Move` _hit (`self.AIPawn`) "CD_North" false))
          (:`Double`
            (bind _aspcontroller (cast `/Game/Blueprints/Controllers/PController` (`self.GetController`)))
            (`/Game/Blueprints/Controllers/PController.Switch Camera` _aspcontroller)))))))

(event `Bean Decremented`
  (params (BeansLeft :type Boolean))
  (`/Game/Blueprints/GUI/Game_HUD.Bean Subtracted` (`self.HUD`) BeansLeft)
  (if (not BeansLeft)
    (set `/Game/Blueprints/Actors/AIPawn.MovePermitted` false (`self.AIPawn`))))

(fn `CallMove`
  (params (Direction :type "ECardinalDir Enum" :default "CD_North"))
  (bind _aipawn (`self.AIPawn`))
  (if (`/Game/Blueprints/Actors/AIPawn.MovePermitted` _aipawn)
    (bind _asaipcontroller (cast `/Game/Blueprints/Controllers/AIPController` (`self.GetController` _aipawn)))
    (if (`/Game/Blueprints/Controllers/AIPController.Grabbing` _asaipcontroller)
      (`/Game/Blueprints/Actors/Pushable_Box.Push` (`/Game/Blueprints/Controllers/AIPController.Grabbed` _asaipcontroller) Direction)
      (else
        (bind _hit (`self.Positional Trace` Direction (`SceneComponent.K2_GetComponentLocation` (`Character.CapsuleComponent` (`self.AIPawn`)))))
        (`self.Perform Move` _hit (`self.AIPawn`) Direction)))))

(fn `Camera Trace`
  (params (`World Location` :type "Vector Structure") (`World Direction` :type "Vector Structure"))
  (returns (Hit :type "Actor Object Reference"))
  (bind _outhit (`KismetSystemLibrary.LineTraceSingle` (`SceneComponent.K2_GetComponentLocation` (`Actor.RootComponent` (`self.ActiveCamera`))) (+ `World Location` (* `World Direction` 10000.0)) "TraceTypeQuery1" false (`self.Beans`)))
  (return (`.HitActor` (`GameplayStatics.BreakHitResult` _outhit))))

(fn `Perform Move`
  (params (`Hit Target` :type "Object Object Reference") (`AI Pawn` :type "/Game/Blueprints/Actors/AIPawn Object Reference") (MovingDir :type "ECardinalDir Enum" :default "CD_North") (`Can Grab Boxes` :type Boolean :default true))
  (bind _aitarget (`self.AITarget`))
  (if (`/Game/Blueprints/Actors/AIPawn.MovePermitted` (`self.AIPawn`))
    (bind _asaipcontroller (cast `/Game/Blueprints/Controllers/AIPController` (`self.GetController` `AI Pawn`)))
    (`/Engine/EditorBlueprintResources/StandardMacros.IsValid` `Hit Target`
      (:`Is Valid`
        (bind _aspushable_box (cast `/Game/Blueprints/Actors/Pushable_Box` `Hit Target`) ; Check if hit object is box
          (:`then`
            (if (`/Game/Blueprints/Actors/Pushable_Box.IsGrabbed` _aspushable_box)
              (bind _location (`/Game/Blueprints/Actors/Pushable_Box.GetWalkPoint` _aspushable_box))
              (set `self.AITarget` _location)
              (if (`/Game/Blueprints/Controllers/AIPController.Grabbing` _asaipcontroller) :!label _label
                (`/Game/Blueprints/Actors/Pushable_Box.Request Release & Move` (`/Game/Blueprints/Controllers/AIPController.Grabbed` _asaipcontroller) true _aitarget)
                (else
                  (`/Game/Blueprints/Controllers/AIPController.MoveChar` _asaipcontroller _aitarget null "CD_North")))
              (elif `Can Grab Boxes`
                (if (`/Game/Blueprints/Actors/Pushable_Box.Grabbable` _aspushable_box)
                  (`/Game/Blueprints/Actors/Pushable_Box.MovePlayerToBox` _aspushable_box _asaipcontroller MovingDir)
                  (else
                    (set `self.AITarget` (`SceneComponent.K2_GetComponentLocation` (`/Game/Blueprints/Actors/Pushable_Box.PlayerTopLoc` _aspushable_box)))
                    (goto _label))))))
          (:`CastFailed`
            (bind _asland_tile (cast `/Game/Blueprints/Actors/LandTile` `Hit Target`))
            (bind _location_2 (`/Game/Blueprints/Actors/LandTile.GetWalkPoint` _asland_tile))
            (set `self.AITarget` _location_2)
            (goto _label)))))))

(fn `Positional Trace`
  (params (Direction :type "ECardinalDir Enum" :default "CD_North") (Location :type "Vector Structure"))
  (returns (Hit :type "Object Object Reference"))
  (locals (TraceOffset :type "Vector Structure"))
  (bind _returnvalue (+ Location (`local.TraceOffset`)))
  ;[1 1 1] Trace from offset location based on direction to 200u below offset location
  (switch `ECardinalDir` Direction
    (:`CD_North`
      (set `local.TraceOffset` (200.0 0.0 0.0)))
    (:`CD_East`
      (set `local.TraceOffset` (0.0 200.0 0.0)))
    (:`CD_South`
      (set `local.TraceOffset` (-200.0 0.0 0.0)))
    (:`CD_West`
      (set `local.TraceOffset` (0.0 -200.0 0.0))))
  (bind _outhit (`KismetSystemLibrary.LineTraceSingle` _returnvalue (+ _returnvalue (0.0 0.0 -200.0)) "TraceTypeQuery1" false (`self.Beans`)))
  (return (`.HitActor` (`GameplayStatics.BreakHitResult` _outhit))))

(fn `Trace From Camera`
  (params (`World Location` :type "Vector Structure") (`World Direction` :type "Vector Structure"))
  (returns (Hit :type "Actor Object Reference"))
  (bind _outhit (`KismetSystemLibrary.LineTraceSingle` (`SceneComponent.K2_GetComponentLocation` (`Actor.RootComponent` (`self.ActiveCamera`))) (+ `World Location` (* `World Direction` 10000.0)) "TraceTypeQuery1"))
  (return (`.HitActor` (`GameplayStatics.BreakHitResult` _outhit))))

(fn `UserConstructionScript`
  (`SceneComponent.K2_SetWorldRotation` (`self.Camera`) (struct :`Pitch` -65.0) false false))