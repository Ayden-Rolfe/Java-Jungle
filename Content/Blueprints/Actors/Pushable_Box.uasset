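; Grid-snapped puzzle box that an AIPawn grabs, attaches to, and pushes or pulls along the grabbed axis.
; Push checks line traces for walls, and for footing when pulling, then Tick interpolates the move linearly with drag particles.
; With no ground beneath, it releases the pawn, becomes ungrabbable and drops with ease-in and a landing effect.
; Releases send the pawn to traced tiles or boxes, whose tops provide walk points.
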(event `self.ReceiveTick`
  (params (DeltaSeconds :type "Float (single-precision)"))
  (bind _targetposition (`self.TargetPosition`))
  (bind (_vector _in_progress _alpha) (`self.Easing Caluclator` DeltaSeconds "EaseIn" (`self.BoxFallTimeDuration`)))
  (bind (_vector_2 _in_progress_2 _alpha_2) (`self.Easing Caluclator` DeltaSeconds "Linear" (`self.BoxPushTimeDuration`)))
  ;[1 1 1] Movement Handling/Tick
  (`|ExecutionSequence`
    (:`then_0`
      (if (`self.BeingPushed`)
        (`self.K2_SetActorLocation` _vector_2)
        (if _in_progress_2
          (set `self.BoxPushTime` _alpha_2)
          (else
            (`ActorComponent.SetActive` (`self.Drag_L`) false false)
            (`ActorComponent.SetActive` (`self.Drag_R`) false false)
            (`self.Set Move Allowed & Being Pushed` true)
            (set `/Game/Blueprints/Actors/AIPawn.State` "NewEnumerator2" (`self.Pawn`))
            (`self.K2_SetActorLocation` _targetposition)
            (bind _ground_available (`self.Trace for ground under this`))
            (if (not _ground_available)
              (`self.Request Release & Move` false)
              (`|ExecutionSequence`
                (:`then_0`
                  (set `self.Over Pit` true)
                  (set `self.Grabbable` false))
                (:`then_1`
                  (`self.Prepare for Push` (`KismetMathLibrary.MakeVector` 0.0 0.0 (* (`self.BoxFallDistance`) -1.0))))))))))
    (:`then_1`
      (if (`self.Over Pit`)
        (`self.K2_SetActorLocation` _vector)
        (if _in_progress
          (set `self.BoxPushTime` _alpha)
          (else
            (set `self.Over Pit` false)
            (`self.K2_SetActorLocation` _targetposition)
            (`GameplayStatics.SpawnEmitterAtLocation` "/Game/ParticleSystems/Boxdrop/P_Box_drop.P_Box_drop" (+ _targetposition (`KismetMathLibrary.MakeVector` 0.0 0.0 (`self.BoxFallDistance`))) (struct) (1.0 1.0 1.0) true "AutoRelease")))))
    (:`then_2`
      (if (`self.BeingPushed`)
        (`SceneComponent.K2_SetRelativeRotation` (`self.PushPullParticleRoot`) (`ExtraMathFunc.GetCardinalDirection` (`self.PushedDir`)) false false)
        (`ActorComponent.SetActive` (`self.Drag_L`) true false)
        (`ActorComponent.SetActive` (`self.Drag_R`) true false)))))

(event `self.ReceiveBeginPlay`
  (`self.K2_SetActorLocation` (`ExtraMathFunc.RoundToNearest` 200.0 (`self.K2_GetActorLocation`) true true)))

(event `Push`
  (params (`Move Direction` :type "ECardinalDir Enum" :default "CD_North"))
  (bind _grabbeddir (`self.GrabbedDir`))
  (bind _grabbeddir_2 (`self.GrabbedDir`))
  (bind _returnvalue (`ExtraMathFunc.GetCardinalOffset` _grabbeddir_2))
  (bind _returnvalue_2 (`ExtraMathFunc.InvertCardinal` (`self.GrabbedDir`)))
  ;[0 0 0] Push logic
  (if (not (`self.BeingPushed`))
    (set `self.PushedDir` `Move Direction`)
    (if (`ExtraMathFunc.IsOnSamePlane` `Move Direction` _grabbeddir)
      (`self.Set Move Allowed & Being Pushed` false)
      (if (`|EnumEquality` _grabbeddir `Move Direction`)
        (bind _hit (`self.Trace for walls` (+ (`SceneComponent.K2_GetComponentLocation` (`self.TraceOrigin`)) (`ExtraMathFunc.VectorMultiplyByAxis` (`ExtraMathFunc.GetCardinalOffset` _grabbeddir_2) 2.0 true true))))
        (if _hit
          (`self.Set Move Allowed & Being Pushed` true :!label _label)
          (else
            (bind _hit_ground (`self.Trace for ground at location` (`ExtraMathFunc.VectorMultiplyByAxis` _returnvalue 2.0 true true)))
            (if _hit_ground
              (set `/Game/Blueprints/Actors/AIPawn.State` "NewEnumerator3" (`self.Pawn`))
              (`self.Prepare for Push` _returnvalue)
              (else
                (goto _label)))))
        (else
          (bind _hit_2 (`self.Trace for walls` (`self.Get Location With Offset` (`self.TraceOrigin`) _returnvalue_2)))
          (if _hit_2
            (goto _label)
            (else
              (set `/Game/Blueprints/Actors/AIPawn.State` "NewEnumerator4" (`self.Pawn`))
              (`self.Prepare for Push` (`ExtraMathFunc.GetCardinalOffset` _returnvalue_2))))))
      (else
        (`self.Request Release & Move` false)))))

(event `AttachToBox`
  (params (Caller :type "/Game/Blueprints/Controllers/AIPController Object Reference") (Direction :type "ECardinalDir Enum" :default "CD_North"))
  (bind _returnvalue (`Controller.K2_GetPawn` Caller))
  ;[0.5492 1 0.6267] Attach player to box
  (`self.TutorialDispatch`)
  (`self.K2_SetActorRotation` _returnvalue (`ExtraMathFunc.GetCardinalDirection` Direction) false)
  (`self.K2_AttachToActor` _returnvalue self "None" "KeepWorld" "KeepWorld" "KeepWorld" true)
  (`|ExecutionSequence`
    (:`then_0`
      (set `/Game/Blueprints/Controllers/AIPController.Grabbing` true Caller)
      (set `self.GrabbedDir` (`ExtraMathFunc.InvertCardinal` Direction)))
    (:`then_1`
      (set `/Game/Blueprints/Controllers/AIPController.Grabbed` self Caller)
      (set `self.IsGrabbed` true))
    (:`then_2`
      (bind _asaipawn (cast `/Game/Blueprints/Actors/AIPawn` _returnvalue))
      (set `self.Pawn` _asaipawn)
      (set `/Game/Blueprints/Actors/AIPawn.MovePermitted` true _asaipawn)
      (set `/Game/Blueprints/Actors/AIPawn.State` "NewEnumerator2" _asaipawn))))

(fn `Attempt Release`
  (returns (Released :type Boolean) (`Go To Space` :type "Vector Structure"))
  (locals (`Can Release` :type Boolean))
  (if (not (`self.BeingPushed`))
    (bind (_location_possible _location) (`self.Trace for ground at grab point`))
    (if _location_possible
      (bind _output_get (set `local.Can Release` true))))
  (return _output_get _location))

(fn `GetWalkPoint`
  (returns (Location :type "Vector Structure"))
  (return (`SceneComponent.K2_GetComponentLocation` (`self.PlayerTopLoc`))))

(fn `MovePlayerToBox`
  (params (AIController :type "/Game/Blueprints/Controllers/AIPController Object Reference") (MoveDir :type "ECardinalDir Enum" :default "CD_North"))
  (locals (Target :type "CapsuleComponent Object Reference"))
  (switch `ECardinalDir` (`ExtraMathFunc.InvertCardinal` MoveDir)
    (:`CD_North`
      (set `local.Target` (`self.PlayerPushNorth`)))
    (:`CD_East`
      (set `local.Target` (`self.PlayerPushEast`)))
    (:`CD_South`
      (set `local.Target` (`self.PlayerPushSouth`)))
    (:`CD_West`
      (set `local.Target` (`self.PlayerPushWest`))))
  (`/Game/Blueprints/Controllers/AIPController.MoveChar` AIController (`SceneComponent.K2_GetComponentLocation` (`local.Target`)) self MoveDir))

(fn `Request Release & Move`
  (params (`Move From Position` :type Boolean) (Position :type "Vector Structure"))
  (`self.K2_DetachFromActor` (`self.Pawn`) "KeepWorld" "KeepWorld" "KeepWorld")
  (bind _asaipcontroller (cast `/Game/Blueprints/Controllers/AIPController` (`Pawn.GetController` (`self.Pawn`))))
  (if `Move From Position`
    (`/Game/Blueprints/Controllers/AIPController.MoveChar` _asaipcontroller Position null "CD_North")
    (else
      (bind (_released _go_to_space) (`self.Attempt Release`))
      (`/Game/Blueprints/Controllers/AIPController.MoveChar` _asaipcontroller _go_to_space null "CD_North")))
  (`|ExecutionSequence`
    (:`then_0`
      (set `/Game/Blueprints/Controllers/AIPController.Grabbing` false _asaipcontroller))
    (:`then_1`
      (set `/Game/Blueprints/Controllers/AIPController.Grabbed` null _asaipcontroller)
      (set `self.IsGrabbed` false))))

(fn `Trace for ground at grab point`
  (returns (`Location Possible` :type Boolean) (Location :type "Vector Structure"))
  (locals (Loc :type "Vector Structure") (LocPossible :type Boolean))
  (bind _returnvalue (+ (`SceneComponent.K2_GetComponentLocation` (`self.TraceOrigin`)) (`ExtraMathFunc.GetCardinalOffset` (`self.GrabbedDir`))))
  (bind _outhit (`KismetSystemLibrary.LineTraceSingle` _returnvalue (- _returnvalue (0.0 0.0 100.0)) "TraceTypeQuery1")) ; Looks for ground to move player to after release
  (bind (_bblockinghit _binitialoverlap _time _distance _location _impactpoint _normal _impactnormal _physmat _hitactor) (`GameplayStatics.BreakHitResult` _outhit))
  (bind _asland_tile (cast `/Game/Blueprints/Actors/LandTile` _hitactor)
    (:`then`
      (bind _location_2 (`/Game/Blueprints/Actors/LandTile.GetWalkPoint` _asland_tile))
      (set `local.Loc` _location_2)
      (set `local.LocPossible` true))
    (:`CastFailed`
      (bind _aspushable_box (cast `/Game/Blueprints/Actors/Pushable_Box` _hitactor)
        (:`then`
          (bind _location_3 (`self.GetWalkPoint` _aspushable_box))
          (set `local.Loc` _location_3)
          (set `local.LocPossible` true))
        (:`CastFailed`
          _))))
  (return (`local.LocPossible`) (`local.Loc`)))

(fn `UserConstructionScript`)